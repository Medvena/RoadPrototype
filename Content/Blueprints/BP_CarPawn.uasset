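; BP_CarPawn is a drivable car pawn with simple kinematic movement instead of physics simulation.
; Enhanced Input sets Steering and Throttle, with IMC_Car registered on BeginPlay.
; Tick eases CurrentSpeed toward the throttle's forward or reverse target at acceleration, brake or deceleration rates, then moves the actor with sweeps.
; Yaw rate scales with speed ratio above a minimum and follows the travel direction's sign, so steering inverts in reverse.
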(event Input|EnhancedActionEvents|EnhancedInputActionIA_MoveForward
  (params (ActionValue :type Float%20%28double-precision%29) (ElapsedSeconds :type Float%20%28double-precision%29) (TriggeredSeconds :type Float%20%28double-precision%29) (InputAction :type Input%20Action%20Object%20Reference :default "/Game/Inputs/IA_MoveForward.IA_MoveForward"))
  ;[0.03036 0.474 0 0.5] Move Up & Down
  (:Triggered
    (Variables|Default|SetThrottle ActionValue))
  (:Completed
    (Variables|Default|SetThrottle 0.0)))

(event Input|EnhancedActionEvents|EnhancedInputActionIA_Turn
  (params (ActionValue :type Float%20%28double-precision%29) (ElapsedSeconds :type Float%20%28double-precision%29) (TriggeredSeconds :type Float%20%28double-precision%29) (InputAction :type Input%20Action%20Object%20Reference :default "/Game/Inputs/IA_Turn.IA_Turn"))
  ;[0.06691 0.5469 0 0.5] Turn
  (:Triggered
    (Variables|Default|SetSteering ActionValue))
  (:Completed
    (Variables|Default|SetSteering 0.0)))

(event EventBeginPlay
  ;[0 0.5104 0.1035 0.5] Add Mapping Context
  (bind _asplayer_controller (Utilities|Casting|CastToPlayerController (Pawn|GetController)))
  (Utilities|IsValid (PlayerController|LocalPlayerSubsystems|GetEnhancedInputLocalPlayerSubsystem _asplayer_controller)
    (:Is%20Valid
      (Input|AddMappingContext (PlayerController|LocalPlayerSubsystems|GetEnhancedInputLocalPlayerSubsystem _asplayer_controller) "/Game/Inputs/IMC_Car.IMC_Car" 0 "(bIgnoreAllPressedKeysUntilRelease=True,bForceImmediately=False,bNotifyUserSettings=False)"))))

(event EventTick
  (params (DeltaSeconds :type Float%20%28single-precision%29))
  ;[0.5938 0.1113 0.1132 0.5] Turn
  (Transformation|AddActorLocalRotation (Math|Rotator|MakeRotator 0.0 0.0 (* DeltaSeconds (* (* (* (Variables|Default|GetSteering) (Variables|Default|GetTurnRate)) (Math|Float|Clamp(Float) (/ (Math|Float|Absolute(Float) (Variables|Default|GetCurrentSpeed)) (Variables|Default|GetMaxSpeed)) (Variables|Default|GetMinSteerRatio))) (Math|Float|Sign(Float) (Variables|Default|GetCurrentSpeed))))) true false)
  ;[0.01345 0.555 0.901 0.5] Forward and Backward
  (if (== (Variables|Default|GetThrottle) 0.0)
    (Variables|Default|SetInterpSpeed (Variables|Default|GetDeceleration))
    (elif (< (* (Math|Float|Sign(Float) (Variables|Default|GetCurrentSpeed)) (Math|Float|Sign(Float) (Variables|Default|GetThrottle))) 0.0)
      (Variables|Default|SetInterpSpeed (Variables|Default|GetBrakeSpeed))
      (else
        (Variables|Default|SetInterpSpeed (Variables|Default|GetAcceleration)))))
  (bind _output_get (Variables|Default|SetCurrentSpeed (Math|Interpolation|FInterptoConstant (Variables|Default|GetCurrentSpeed) (* (select (< (Variables|Default|GetThrottle) 0.0) (Variables|Default|GetMaxReverseSpeed) (Variables|Default|GetMaxSpeed)) (Variables|Default|GetThrottle)) DeltaSeconds (Variables|Default|GetInterpSpeed))))
  (Transformation|AddActorLocalOffset (Math|Vector|MakeVector (* _output_get DeltaSeconds) 0.0 0.0) true false))

(fn ConstructionScript)